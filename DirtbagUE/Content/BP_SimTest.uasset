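; BP_SimTest is a test actor that runs a single climbing attempt through the simulation on BeginPlay.
; It builds a seeded power boulder route and starts a session with a hard-coded, high-stat powerful climber, storing it in Session.
; It then runs one attempt using that session, Memory, an identical climber and the route, and prints the highpoint and send result on screen.
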(event EventBeginPlay
  (bind _returnvalue (Class|DirtbagSimLibrary|BuildRoute "gym-1" "First Blood" 11 12 "Power" "Boulder"))
  (bind _returnvalue_2 (Class|DirtbagSimLibrary|StartSession (Utilities|Struct|MakeDirtbagClimber 9e+01 9e+01 9e+01 9e+01 9e+01 "Powerful")))
  (bind _output_get (Variables|Default|SetSession _returnvalue_2))
  (bind _returnvalue_3 (Class|DirtbagSimLibrary|AttemptinSession "gym-1" _output_get (Variables|Default|GetMemory) (Utilities|Struct|MakeDirtbagClimber 9e+01 9e+01 9e+01 9e+01 9e+01 "Powerful") _returnvalue 0.5 0.72))
  (Development|PrintString (Utilities|String|ToString(Integer) (.Highpoint (Utilities|Struct|BreakDirtbagAttemptResult _returnvalue_3))) true true "(R=0.000000,G=0.660000,B=1.000000,A=1.000000)" 1e+01)
  (Development|PrintString (Utilities|String|ToString(Boolean) (.bSent (Utilities|Struct|BreakDirtbagAttemptResult _returnvalue_3))) true true "(R=0.000000,G=0.660000,B=1.000000,A=1.000000)" 1e+01))

(event Collision|EventActorBeginOverlap
  (params (OtherActor :type Actor%20Object%20Reference)))

(event EventTick
  (params (DeltaSeconds :type Float%20%28single-precision%29)))

(fn ConstructionScript)